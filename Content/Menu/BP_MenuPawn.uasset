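; Menu pawn that shows the cursor and start-work widget, then moves its camera between menu screens.
; MoveToComputer and MoveToUpgrade clear the current UI, pause briefly, move the camera to a marker component, then open the computer or upgrades widget.
; The upgrade move also rotates the camera by offsetting its forward vector.
; The UI-only input mode call is unconnected, and MoveCameraStartWork is empty.
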(event `self.ReceiveBeginPlay`
  (set `PlayerController.bShowMouseCursor` true (`GameplayStatics.GetPlayerController` 0))
  (bind _returnvalue (`|CreateWidget` "/Game/Menu/Widgets/WB_StartWork.WB_StartWork_C"))
  (bind _output_get (set `self.StartWorkUI` _returnvalue))
  (`UserWidget.AddToViewport` _output_get 0))

(event `MoveToComputer`
  (`Widget.RemoveFromParent` (`self.StartWorkUI`))
  (`KismetSystemLibrary.Delay` 0.5)
  (`KismetSystemLibrary.MoveComponentTo` (`self.Camera`) (`SceneComponent.RelativeLocation` (`self.MoveTo`)) (struct) true true 2.0)
  (bind _returnvalue (`|CreateWidget` "/Game/Menu/Widgets/WB_ComputerScreenMain.WB_ComputerScreenMain_C"))
  (bind _output_get (set `self.ComputerMainScreen` _returnvalue))
  (`UserWidget.AddToViewport` _output_get 0))

(event `MoveToUpgrade`
  (`WidgetLayoutLibrary.RemoveAllWidgets`)
  (`KismetSystemLibrary.Delay` 0.2)
  (`KismetSystemLibrary.MoveComponentTo` (`self.Camera`) (`SceneComponent.RelativeLocation` (`self.MoveTo_02`)) (`KismetMathLibrary.Conv_VectorToRotator` (+ (`KismetMathLibrary.GetAxes` (`SceneComponent.RelativeRotation` (`self.Camera`))) (`self.RotationValue`))) false false 2.0)
  (bind _returnvalue (`|CreateWidget` "/Game/Menu/Widgets/WB_Upgrades.WB_Upgrades_C"))
  (bind _output_get (set `self.Upgrades Widget` _returnvalue))
  (`UserWidget.AddToViewport` _output_get 0))

(fn `MoveCameraStartWork`)

(fn `UserConstructionScript`)